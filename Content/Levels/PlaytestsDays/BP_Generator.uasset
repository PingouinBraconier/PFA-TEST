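; Generator actor with four plates, one of which becomes interactive on day 1, 4, 5 or 7.
; BeginPlay reads the player's DayNumber, sets the matching flag and disables collision on the other three plates.
; Looking at it highlights the active plate's meshes and flags the player until a short retriggerable delay expires; the first also shows ItemRef.
; Interacting only affects the day 1 panel, swinging it open or closed through a flip-flopped timeline.
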(event `self.ReceiveBeginPlay`
  (bind _asbp_first_person_character (cast `/Game/Characters/Character/Blueprints/BP_FirstPersonCharacter` (`GameplayStatics.GetPlayerPawn` 0)))
  (set `self.As BP First Person Character Ref` _asbp_first_person_character)
  (if (== (`/Game/Characters/Character/Blueprints/BP_FirstPersonCharacter.DayNumber` (`self.As BP First Person Character Ref`)) 1)
    (set `self.Interactive1` true)
    (`PrimitiveComponent.SetCollisionEnabled` (`self.Plate2`) "NoCollision")
    (`PrimitiveComponent.SetCollisionEnabled` (`self.Plate7`) "NoCollision")
    (`PrimitiveComponent.SetCollisionEnabled` (`self.Plate8`) "NoCollision")
    (elif (== (`/Game/Characters/Character/Blueprints/BP_FirstPersonCharacter.DayNumber` (`self.As BP First Person Character Ref`)) 4)
      (set `self.Interactive2` true)
      (`PrimitiveComponent.SetCollisionEnabled` (`self.Plate1`) "NoCollision")
      (`PrimitiveComponent.SetCollisionEnabled` (`self.Plate7`) "NoCollision")
      (`PrimitiveComponent.SetCollisionEnabled` (`self.Plate8`) "NoCollision")
      (elif (== (`/Game/Characters/Character/Blueprints/BP_FirstPersonCharacter.DayNumber` (`self.As BP First Person Character Ref`)) 5)
        (set `self.Interactive3` true)
        (`PrimitiveComponent.SetCollisionEnabled` (`self.Plate1`) "NoCollision")
        (`PrimitiveComponent.SetCollisionEnabled` (`self.Plate8`) "NoCollision")
        (`PrimitiveComponent.SetCollisionEnabled` (`self.Plate2`) "NoCollision")
        (elif (== (`/Game/Characters/Character/Blueprints/BP_FirstPersonCharacter.DayNumber` (`self.As BP First Person Character Ref`)) 7)
          (set `self.Interactive4` true)
          (`PrimitiveComponent.SetCollisionEnabled` (`self.Plate7`) "NoCollision")
          (`PrimitiveComponent.SetCollisionEnabled` (`self.Plate2`) "NoCollision")
          (`PrimitiveComponent.SetCollisionEnabled` (`self.Plate1`) "NoCollision"))))))

(event `/Game/Blueprints/Interfaces/BPI_Interaction.OnInteract`
  (params (InteractingPlayer :type "Character Object Reference"))
  (if (`self.Interactive1`)
    (`/Engine/EditorBlueprintResources/StandardMacros.FlipFlop`
      (:`A`
        (bind (_direction _open) (`Timeline|Open` :!label _label)
          (:`Update`
            (`SceneComponent.K2_SetRelativeRotation` (`self.Scene1`) (`KismetMathLibrary.RLerp` (struct) (struct :`Roll` -130.0) _open) false false))))
      (:`B`
        (goto _label :!via `Reverse`)))))

(event `/Game/Blueprints/Interfaces/BPI_Interaction.OnLookAt`
  (params (Actor :type "Actor Object Reference"))
  (if (`self.Interactive1`)
    (`MeshComponent.SetOverlayMaterial` (`self.Plate1`) "/Game/Materials/M_Overlay.M_Overlay")
    (`MeshComponent.SetOverlayMaterial` (`self.StaticMesh2`) "/Game/Materials/M_Overlay.M_Overlay")
    (`MeshComponent.SetOverlayMaterial` (`self.StaticMesh3`) "/Game/Materials/M_Overlay.M_Overlay")
    (`MeshComponent.SetOverlayMaterial` (`self.StaticMesh`) "/Game/Materials/M_Overlay.M_Overlay")
    (`MeshComponent.SetOverlayMaterial` (`self.StaticMesh1`) "/Game/Materials/M_Overlay.M_Overlay")
    (`SceneComponent.SetVisibility` (`self.ItemRef`) true false)
    (set `/Game/Characters/Character/Blueprints/BP_FirstPersonCharacter.LookAtBool` true (`self.As BP First Person Character Ref`))
    (`KismetSystemLibrary.RetriggerableDelay` 0.11)
    (`MeshComponent.SetOverlayMaterial` (`self.Plate1`) null)
    (`MeshComponent.SetOverlayMaterial` (`self.StaticMesh1`) null)
    (`MeshComponent.SetOverlayMaterial` (`self.StaticMesh`) null)
    (`MeshComponent.SetOverlayMaterial` (`self.StaticMesh3`) null)
    (`MeshComponent.SetOverlayMaterial` (`self.StaticMesh2`) null)
    (set `/Game/Characters/Character/Blueprints/BP_FirstPersonCharacter.LookAtBool` false (`self.As BP First Person Character Ref`))
    (`SceneComponent.SetVisibility` (`self.ItemRef`) false false)
    (elif (`self.Interactive2`)
      (`MeshComponent.SetOverlayMaterial` (`self.StaticMesh5`) "/Game/Materials/M_Overlay.M_Overlay")
      (`MeshComponent.SetOverlayMaterial` (`self.StaticMesh4`) "/Game/Materials/M_Overlay.M_Overlay")
      (`MeshComponent.SetOverlayMaterial` (`self.StaticMesh7`) "/Game/Materials/M_Overlay.M_Overlay")
      (`MeshComponent.SetOverlayMaterial` (`self.StaticMesh6`) "/Game/Materials/M_Overlay.M_Overlay")
      (`MeshComponent.SetOverlayMaterial` (`self.Plate2`) "/Game/Materials/M_Overlay.M_Overlay")
      (set `/Game/Characters/Character/Blueprints/BP_FirstPersonCharacter.LookAtBool` true (`self.As BP First Person Character Ref`))
      (`KismetSystemLibrary.RetriggerableDelay` 0.11)
      (`MeshComponent.SetOverlayMaterial` (`self.StaticMesh5`) null)
      (`MeshComponent.SetOverlayMaterial` (`self.StaticMesh4`) null)
      (`MeshComponent.SetOverlayMaterial` (`self.StaticMesh7`) null)
      (`MeshComponent.SetOverlayMaterial` (`self.StaticMesh6`) null)
      (`MeshComponent.SetOverlayMaterial` (`self.Plate2`) null)
      (set `/Game/Characters/Character/Blueprints/BP_FirstPersonCharacter.LookAtBool` false (`self.As BP First Person Character Ref`))
      (elif (`self.Interactive3`)
        (`MeshComponent.SetOverlayMaterial` (`self.StaticMesh25`) "/Game/Materials/M_Overlay.M_Overlay")
        (`MeshComponent.SetOverlayMaterial` (`self.StaticMesh24`) "/Game/Materials/M_Overlay.M_Overlay")
        (`MeshComponent.SetOverlayMaterial` (`self.StaticMesh27`) "/Game/Materials/M_Overlay.M_Overlay")
        (`MeshComponent.SetOverlayMaterial` (`self.StaticMesh26`) "/Game/Materials/M_Overlay.M_Overlay")
        (`MeshComponent.SetOverlayMaterial` (`self.Plate7`) "/Game/Materials/M_Overlay.M_Overlay")
        (set `/Game/Characters/Character/Blueprints/BP_FirstPersonCharacter.LookAtBool` true (`self.As BP First Person Character Ref`))
        (`KismetSystemLibrary.RetriggerableDelay` 0.11)
        (`MeshComponent.SetOverlayMaterial` (`self.Plate7`) null)
        (`MeshComponent.SetOverlayMaterial` (`self.StaticMesh25`) null)
        (`MeshComponent.SetOverlayMaterial` (`self.StaticMesh24`) null)
        (`MeshComponent.SetOverlayMaterial` (`self.StaticMesh27`) null)
        (`MeshComponent.SetOverlayMaterial` (`self.StaticMesh26`) null)
        (set `/Game/Characters/Character/Blueprints/BP_FirstPersonCharacter.LookAtBool` false (`self.As BP First Person Character Ref`))
        (elif (`self.Interactive4`)
          (`MeshComponent.SetOverlayMaterial` (`self.Plate8`) "/Game/Materials/M_Overlay.M_Overlay")
          (`MeshComponent.SetOverlayMaterial` (`self.StaticMesh30`) "/Game/Materials/M_Overlay.M_Overlay")
          (`MeshComponent.SetOverlayMaterial` (`self.StaticMesh31`) "/Game/Materials/M_Overlay.M_Overlay")
          (`MeshComponent.SetOverlayMaterial` (`self.StaticMesh28`) "/Game/Materials/M_Overlay.M_Overlay")
          (`MeshComponent.SetOverlayMaterial` (`self.StaticMesh29`) "/Game/Materials/M_Overlay.M_Overlay")
          (set `/Game/Characters/Character/Blueprints/BP_FirstPersonCharacter.LookAtBool` true (`self.As BP First Person Character Ref`))
          (`KismetSystemLibrary.RetriggerableDelay` 0.11)
          (`MeshComponent.SetOverlayMaterial` (`self.Plate8`) null)
          (`MeshComponent.SetOverlayMaterial` (`self.StaticMesh30`) null)
          (`MeshComponent.SetOverlayMaterial` (`self.StaticMesh31`) null)
          (`MeshComponent.SetOverlayMaterial` (`self.StaticMesh28`) null)
          (`MeshComponent.SetOverlayMaterial` (`self.StaticMesh29`) null)
          (set `/Game/Characters/Character/Blueprints/BP_FirstPersonCharacter.LookAtBool` false (`self.As BP First Person Character Ref`)))))))

(fn `UserConstructionScript`)