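; BP_Dust is an interactable dust pile, filed under tasks, that the player can clean up once they have obtained the broom.
; It caches the first-person character on BeginPlay and checks its BroomObtained flag in OnInteract.
; With the broom, a DoOnce gate plays the sweep sound and destroys the actor after a short delay.
; Without it, a WBP_BroomNeeded widget appears briefly on screen.
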(event `self.ReceiveBeginPlay`
  (bind _asbp_first_person_character (cast `/Game/Characters/Character/Blueprints/BP_FirstPersonCharacter` (`GameplayStatics.GetPlayerPawn` 0)))
  (set `self.As BP First Person Character Ref` _asbp_first_person_character))

(event `/Game/Blueprints/InteractiveObjects/BPI_Interaction.OnInteract`
  (params (InteractingPlayer :type "Character Object Reference"))
  (if (`/Game/Characters/Character/Blueprints/BP_FirstPersonCharacter.BroomObtained` (`self.As BP First Person Character Ref`))
    (`/Engine/EditorBlueprintResources/StandardMacros.DoOnce` false
      (:`Completed`
        (`GameplayStatics.PlaySound2D` "/Game/SoundDesign/BroomUsed.BroomUsed" 1.0 1.0 0.0 null null)
        (`KismetSystemLibrary.Delay` 1.5)
        (`self.K2_DestroyActor`)))
    (else
      (bind _returnvalue (`|CreateWidget` "/Game/Widgets/InteractText/WBP_BroomNeeded.WBP_BroomNeeded_C"))
      (`UserWidget.AddToViewport` _returnvalue 0)
      (`KismetSystemLibrary.Delay` 3.0)
      (`Widget.RemoveFromParent` _returnvalue))))

(fn `UserConstructionScript`)