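; BP_Asteroid is a rotating asteroid actor that travels from its starting position to the location of its Sphere component.
; On BeginPlay it caches both endpoints and the first-person character, assigns the Asteroid to RotatingMovement, and starts a looping poll timer.
; The timer plays the Fly timeline while the player is outside the pod and stops it while inside.
; Timeline updates lerp the Asteroid's world position without sweep.
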(event `self.ReceiveBeginPlay`
  (bind _asbp_first_person_character (cast `/Game/Characters/Character/Blueprints/BP_FirstPersonCharacter` (`GameplayStatics.GetPlayerPawn` 0)))
  (set `self.As BP First Person Character Ref` _asbp_first_person_character)
  (`MovementComponent.SetUpdatedComponent` (`self.RotatingMovement`) (`self.Asteroid`))
  (set `self.StartLocation` (`SceneComponent.K2_GetComponentLocation` (`self.Asteroid`)))
  (set `self.EndLocation` (`SceneComponent.K2_GetComponentLocation` (`self.Sphere`)))
  (`KismetSystemLibrary.K2_SetTimerDelegate` (delegate `Pod`) 0.2 true))

(event `Pod`
  (if (`/Game/Characters/Character/Blueprints/BP_FirstPersonCharacter.IsInThePod` (`self.As BP First Person Character Ref`))
    (bind (_direction _fly) (`Timeline|Fly` :!via `Stop` :!label _label)
      (:`Update`
        (`SceneComponent.K2_SetWorldLocation` (`self.Asteroid`) (`KismetMathLibrary.VLerp` (`self.StartLocation`) (`self.EndLocation`) _fly) false false)))
    (else
      (goto _label))))

(fn `UserConstructionScript`)