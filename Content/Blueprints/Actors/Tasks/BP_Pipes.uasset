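; Leaking pipe task actor that the player repairs with tape.
; A looping timer plays a gas-leak sound at the pipe until it is fixed.
; Interacting with tape obtained runs once, triggering the character's Fix and, after a delay, stopping the leak visuals and replacing the actor with BP_ScotchPipes.
; Look-at shows an overlay material and item hint, cleared by a retriggerable delay when gaze leaves.
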(event `self.ReceiveBeginPlay`
  (bind _asbp_first_person_character (cast `/Game/Characters/Character/Blueprints/BP_FirstPersonCharacter` (`GameplayStatics.GetPlayerPawn` 0)))
  (set `self.As BP First Person Character Ref` _asbp_first_person_character)
  (set `self.PipeRef` self)
  (`KismetSystemLibrary.K2_SetTimerDelegate` (delegate `Mute`) 0.5 true))

(event `Mute`
  (if (not (`self.IsFixed`))
    (`GameplayStatics.PlaySoundAtLocation` "/Game/SoundDesign/Tasks/SC_GasLeak.SC_GasLeak" (`self.K2_GetActorLocation` (`self.PipeRef`)) (struct) 0.5 1.0 0.0 null null null null)))

(event `/Game/Blueprints/Interfaces/BPI_Interaction.OnInteract`
  (params (InteractingPlayer :type "Character Object Reference"))
  (if (`/Game/Characters/Character/Blueprints/BP_FirstPersonCharacter.TapeObtained` (`self.As BP First Person Character Ref`))
    (`/Engine/EditorBlueprintResources/StandardMacros.DoOnce` false
      (:`Completed`
        (`/Game/Characters/Character/Blueprints/BP_FirstPersonCharacter.Fix` (`self.As BP First Person Character Ref`))
        (`GameplayStatics.PlaySound2D` "/Game/SoundDesign/Tasks/TapeUsed.TapeUsed" 1.0 1.0 0.0 null null)
        (`KismetSystemLibrary.Delay` 3.5)
        (`SceneComponent.SetVisibility` (`self.Decal`) false false)
        (`ActorComponent.Deactivate` (`self.Niagara`))
        (`SceneComponent.SetVisibility` (`self.Ribbon`) true false)
        (set `self.IsFixed` true)
        (`|SpawnActorFromClass` "/Game/Blueprints/Actors/Tasks/BP_ScotchPipes.BP_ScotchPipes_C" (`self.GetTransform`) "Undefined" "MultiplyWithRoot" null null)
        (`self.K2_DestroyActor`)))))

(event `/Game/Blueprints/Interfaces/BPI_Interaction.OnLookAt`
  (params (Actor :type "Actor Object Reference"))
  (`MeshComponent.SetOverlayMaterial` (`self.Cylinder`) "/Game/Materials/M_Overlay.M_Overlay")
  (`SceneComponent.SetVisibility` (`self.ItemRef`) true false)
  (`KismetSystemLibrary.RetriggerableDelay` 0.11)
  (`MeshComponent.SetOverlayMaterial` (`self.Cylinder`) null)
  (`SceneComponent.SetVisibility` (`self.ItemRef`) false false))

(fn `UserConstructionScript`)