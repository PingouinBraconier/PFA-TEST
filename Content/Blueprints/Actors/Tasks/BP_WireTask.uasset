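; BP_WireTask is an interactable wire task station that moves the player into and out of a fixed screen view.
; Interacting toggles a blend to the BP_WireCam1 camera, freezing walking and look input, hiding cursor widgets and showing the mouse.
; The next interaction blends back to the character and restores movement, game-only input and the crosshair widget.
; Looking at it briefly shows ItemRef, kept visible by a retriggerable delay.
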(event `self.OnInteract`
  (params (InteractingPlayer :type "Character Object Reference"))
  (bind _returnvalue (`GameplayStatics.GetPlayerController` 0))
  (bind _in_widget_to_focus (`self.In Widget to Focus`))
  (`/Engine/EditorBlueprintResources/StandardMacros.FlipFlop`
    (:`A`
      (set `/Game/Characters/Character/Blueprints/BP_FirstPersonCharacter.OnAScreen` true (stale `self.ReceiveBeginPlay` _asbp_first_person_character))
      (`PlayerController.SetViewTargetWithBlend` _returnvalue (stale `self.ReceiveBeginPlay` _returnvalue) 0.5 "VTBlend_EaseInOut" 2.0 false)
      (`WidgetBlueprintLibrary.SetInputMode_GameAndUIEx` _returnvalue _in_widget_to_focus "DoNotLock" false)
      (set `CharacterMovementComponent.MaxWalkSpeed` 0.0 (`Character.CharacterMovement` (`self.As BP First Person Character`)))
      (`Controller.SetIgnoreLookInput` _returnvalue true)
      (bind _foundwidgets (`WidgetBlueprintLibrary.GetAllWidgetsOfClass` "/Game/Widgets/HUD/WBP_Cursor.WBP_Cursor_C"))
      (`Widget.SetVisibility` _foundwidgets "Hidden")
      (set `PlayerController.bShowMouseCursor` true _returnvalue))
    (:`B`
      (set `/Game/Characters/Character/Blueprints/BP_FirstPersonCharacter.OnAScreen` false (stale `self.ReceiveBeginPlay` _asbp_first_person_character))
      (if (not (`/Game/Characters/Character/Blueprints/BP_FirstPersonCharacter.OnAScreen` (stale `self.ReceiveBeginPlay` _asbp_first_person_character)))
        (`PlayerController.SetViewTargetWithBlend` _returnvalue (stale `self.ReceiveBeginPlay` _asbp_first_person_character) 0.5 "VTBlend_EaseInOut" 2.0 false)
        (`WidgetBlueprintLibrary.SetInputMode_GameAndUIEx` _returnvalue _in_widget_to_focus "DoNotLock" false)
        (set `CharacterMovementComponent.MaxWalkSpeed` 500.0 (`Character.CharacterMovement` (`self.As BP First Person Character`)))
        (`KismetSystemLibrary.Delay` 0.5)
        (bind _foundwidgets_2 (`WidgetBlueprintLibrary.GetAllWidgetsOfClass` "/Game/Widgets/HUD/WBP_Cursor.WBP_Cursor_C"))
        (`Widget.SetVisibility` _foundwidgets_2 "Visible")
        (`WidgetBlueprintLibrary.SetInputMode_GameOnly` _returnvalue)
        (`Controller.SetIgnoreLookInput` _returnvalue false)
        (set `PlayerController.bShowMouseCursor` false _returnvalue)))))

(event `self.ReceiveBeginPlay`
  (bind _asbp_first_person_character (cast `/Game/Characters/Character/Blueprints/BP_FirstPersonCharacter` (`GameplayStatics.GetPlayerPawn` 0)))
  (set `self.As BP First Person Character` _asbp_first_person_character)
  (bind _returnvalue (`GameplayStatics.GetActorOfClass` "/Game/Blueprints/Actors/Camera/BP_WireCam1.BP_WireCam1_C")))

(event `/Game/Blueprints/Interfaces/BPI_Interaction.OnLookAt`
  (params (Actor :type "Actor Object Reference"))
  (`SceneComponent.SetVisibility` (`self.ItemRef`) true false)
  (`KismetSystemLibrary.RetriggerableDelay` 0.11)
  (`SceneComponent.SetVisibility` (`self.ItemRef`) false false))

(fn `UserConstructionScript`)