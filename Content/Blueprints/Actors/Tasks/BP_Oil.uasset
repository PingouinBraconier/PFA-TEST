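; BP_Oil is an oil spill task actor that the player cleans up once they have obtained the broom.
; Interacting triggers the character's Clean, a water sound and the Vape effect, while a timeline shrinks the Plane before delayed hiding and self-destruction.
; Being looked at shows ItemRef and an overlay material, cleared by a retriggerable delay once the look events stop.
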(event `self.ReceiveBeginPlay`
  (bind _asbp_first_person_character (cast `/Game/Characters/Character/Blueprints/BP_FirstPersonCharacter` (`GameplayStatics.GetPlayerPawn` 0)))
  (set `self.As BP First Person Character Ref` _asbp_first_person_character))

(event `/Game/Blueprints/Interfaces/BPI_Interaction.OnInteract`
  (params (InteractingPlayer :type "Character Object Reference"))
  (bind _vape (`self.Vape`))
  (if (`/Game/Characters/Character/Blueprints/BP_FirstPersonCharacter.BroomObtained` (`self.As BP First Person Character Ref`))
    (`/Engine/EditorBlueprintResources/StandardMacros.DoOnce` false
      (:`Completed`
        (`/Game/Characters/Character/Blueprints/BP_FirstPersonCharacter.Clean` (`self.As BP First Person Character Ref`))
        (`GameplayStatics.PlaySound2D` "/Game/SoundDesign/Tasks/WaterClean.WaterClean" 0.5 1.0 0.0 null null)
        (`ActorComponent.Activate` (`self.Vape`) false)
        (bind (_direction _cleaning) (`Timeline|Cleaning` :!via `PlayFromStart`)
          (:`Update`
            (`SceneComponent.SetRelativeScale3D` (`self.Plane`) (`KismetMathLibrary.VLerp` (1.0 1.0 0.025) (0.0 0.0 0.025) _cleaning))
            (`KismetSystemLibrary.Delay` 2.0)
            (`SceneComponent.SetVisibility` (`self.Plane`) false false)
            (`SceneComponent.SetVisibility` _vape false false)
            (`ActorComponent.Deactivate` _vape)
            (`KismetSystemLibrary.Delay` 1.0)
            (`self.K2_DestroyActor`)))))))

(event `/Game/Blueprints/Interfaces/BPI_Interaction.OnLookAt`
  (params (Actor :type "Actor Object Reference"))
  (`SceneComponent.SetVisibility` (`self.ItemRef`) true false)
  (`MeshComponent.SetOverlayMaterial` (`self.Plane`) "/Game/Materials/M_Overlay.M_Overlay")
  (`KismetSystemLibrary.RetriggerableDelay` 0.11)
  (`SceneComponent.SetVisibility` (`self.ItemRef`) false false)
  (`MeshComponent.SetOverlayMaterial` (`self.Plane`) null))

(fn `UserConstructionScript`)