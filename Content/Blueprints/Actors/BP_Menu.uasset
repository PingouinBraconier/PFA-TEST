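; BP_Menu is an interactable actor that switches the player between first-person play and a screen camera view.
; BeginPlay caches the BP_FirstPersonCharacter pawn and finds the BP_CamScreen actor in the level.
; OnInteract uses a FlipFlop to blend the view to that camera with cursor and Game-and-UI input, then back to the character with game-only input.
; Each toggle also updates the character's OnAScreen flag.
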(event `self.OnInteract`
  (params (InteractingPlayer :type "Character Object Reference"))
  (bind _returnvalue (`GameplayStatics.GetPlayerController` 0))
  (`/Engine/EditorBlueprintResources/StandardMacros.FlipFlop`
    (:`A`
      (set `/Game/Characters/Character/Blueprints/BP_FirstPersonCharacter.OnAScreen` true (stale `self.ReceiveBeginPlay` _asbp_first_person_character))
      (`PlayerController.SetViewTargetWithBlend` _returnvalue (stale `self.ReceiveBeginPlay` _returnvalue) 0.5 "VTBlend_EaseInOut" 2.0 false)
      (`WidgetBlueprintLibrary.SetInputMode_GameAndUIEx` _returnvalue (`self.In Widget to Focus`))
      (set `PlayerController.bShowMouseCursor` true _returnvalue))
    (:`B`
      (set `/Game/Characters/Character/Blueprints/BP_FirstPersonCharacter.OnAScreen` false (stale `self.ReceiveBeginPlay` _asbp_first_person_character))
      (if (not (`/Game/Characters/Character/Blueprints/BP_FirstPersonCharacter.OnAScreen` (stale `self.ReceiveBeginPlay` _asbp_first_person_character)))
        (`PlayerController.SetViewTargetWithBlend` _returnvalue (stale `self.ReceiveBeginPlay` _asbp_first_person_character) 0.5 "VTBlend_EaseInOut" 2.0 false)
        (`WidgetBlueprintLibrary.SetInputMode_GameOnly` _returnvalue)
        (set `PlayerController.bShowMouseCursor` false _returnvalue)))))

(event `self.ReceiveBeginPlay`
  (bind _asbp_first_person_character (cast `/Game/Characters/Character/Blueprints/BP_FirstPersonCharacter` (`GameplayStatics.GetPlayerPawn` 0)))
  (bind _returnvalue (`GameplayStatics.GetActorOfClass` "/Game/Blueprints/Actors/BP_CamScreen.BP_CamScreen_C")))

(fn `UserConstructionScript`)