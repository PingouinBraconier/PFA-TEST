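; BP_ScotchGiver is an actor that animates two mesh parts when the first-person character enters its trigger sphere, judging by the name to offer scotch.
; A timeline lerps both static meshes' roll, Y and Z in mirrored motion, and reverses when the character leaves.
; CanTake turns true when the timeline finishes and false on exit; this graph only sets the flag and never reads it.
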(event `self.Sphere.OnComponentBeginOverlap`
  (params (OverlappedComponent :type "PrimitiveComponent Object Reference") (OtherActor :type "Actor Object Reference") (OtherComp :type "PrimitiveComponent Object Reference") (OtherBodyIndex :type Integer) (bFromSweep :type Boolean) (SweepResult :type "HitResult Structure (by ref)"))
  (cast `/Game/Characters/Character/Blueprints/BP_FirstPersonCharacter` OtherActor)
  (bind (_direction _newtrack_0) (`Timeline|Timeline` :!label _label)
    (:`Update`
      (`|ExecutionSequence`
        (:`then_0`
          (`SceneComponent.K2_SetRelativeRotation` (`self.StaticMesh1`) (`KismetMathLibrary.MakeRotator` (`KismetMathLibrary.Lerp` -90.0 -180.0 _newtrack_0)) false false)
          (`SceneComponent.K2_SetRelativeRotation` (`self.StaticMesh`) (`KismetMathLibrary.MakeRotator` (`KismetMathLibrary.Lerp` 90.0 180.0 _newtrack_0)) false false))
        (:`then_1`
          (`SceneComponent.K2_SetRelativeLocation` (`self.StaticMesh1`) (`KismetMathLibrary.MakeVector` 0.0 (`KismetMathLibrary.Lerp` -18.0 0.0 _newtrack_0) (`KismetMathLibrary.Lerp` 109.0 94.0 _newtrack_0)) false false)
          (`SceneComponent.K2_SetRelativeLocation` (`self.StaticMesh`) (`KismetMathLibrary.MakeVector` 0.0 (`KismetMathLibrary.Lerp` 17.0 0.0 _newtrack_0) (`KismetMathLibrary.Lerp` 109.0 94.0 _newtrack_0)) false false))))
    (:`Finished`
      (set `self.CanTake` true))))

(event `self.Sphere.OnComponentEndOverlap`
  (params (OverlappedComponent :type "PrimitiveComponent Object Reference") (OtherActor :type "Actor Object Reference") (OtherComp :type "PrimitiveComponent Object Reference") (OtherBodyIndex :type Integer))
  (cast `/Game/Characters/Character/Blueprints/BP_FirstPersonCharacter` OtherActor)
  (set `self.CanTake` false)
  (goto _label :!via `Reverse`))

(fn `UserConstructionScript`)