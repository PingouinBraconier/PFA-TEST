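; BP_Light is an actor whose point light cycles through rainbow colors, from red to violet, for as long as it runs.
; BeginPlay starts a custom event that steps the PointLight color at fixed half-second delays.
; The event calls itself after the last color to loop endlessly, with hard switches rather than blending.
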(event `self.ReceiveBeginPlay`
  (`self.CustomEvent`))

(event `CustomEvent`
  (`LightComponent.SetLightColor` (`self.PointLight`) (struct :`R` 1.0 :`A` 1.0) true)
  (`KismetSystemLibrary.Delay` 0.5)
  (`LightComponent.SetLightColor` (`self.PointLight`) (struct :`R` 1.0 :`G` 0.332472 :`A` 1.0) true)
  (`KismetSystemLibrary.Delay` 0.5)
  (`LightComponent.SetLightColor` (`self.PointLight`) (struct :`R` 1.0 :`G` 0.863269 :`A` 1.0) true)
  (`KismetSystemLibrary.Delay` 0.5)
  (`LightComponent.SetLightColor` (`self.PointLight`) (struct :`R` 0.07169 :`G` 1.0 :`A` 1.0) true)
  (`KismetSystemLibrary.Delay` 0.5)
  (`LightComponent.SetLightColor` (`self.PointLight`) (struct :`R` 0.000133 :`G` 0.241994 :`B` 1.0 :`A` 1.0) true)
  (`KismetSystemLibrary.Delay` 0.5)
  (`LightComponent.SetLightColor` (`self.PointLight`) (struct :`R` 0.579126 :`B` 1.0 :`A` 1.0) true)
  (`KismetSystemLibrary.Delay` 0.5)
  (`self.CustomEvent`))

(fn `UserConstructionScript`)