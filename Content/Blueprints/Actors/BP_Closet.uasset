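; BP_Closet is an interactable closet whose two doors alternately swing open and closed on each OnInteract.
; A FlipFlop picks one of two timelines, each lerping the yaw of the left and right pivot cylinders in opposite directions.
; A DoOnce guards the input but resets on every timeline Update rather than on completion, so it barely blocks interaction mid-swing.
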(event `/Game/Blueprints/InteractiveObjects/BPI_Interaction.OnInteract`
  (params (InteractingPlayer :type "Character Object Reference"))
  (`/Engine/EditorBlueprintResources/StandardMacros.DoOnce` false :!label _label
    (:`Completed`
      (`KismetSystemLibrary.PrintString` "INTERACTION")
      (`/Engine/EditorBlueprintResources/StandardMacros.FlipFlop`
        (:`A`
          (bind (_direction _opencloset) (`Timeline|Timeline`)
            (:`Update`
              (`SceneComponent.K2_SetRelativeRotation` (`self.CylinderToRotateLeft`) (`KismetMathLibrary.MakeRotator` 0.0 0.0 (`KismetMathLibrary.Lerp` 0.0 130.0 _opencloset)) false false)
              (`SceneComponent.K2_SetRelativeRotation` (`self.CylinderToRotateRight`) (`KismetMathLibrary.MakeRotator` 0.0 0.0 (`KismetMathLibrary.Lerp` -92.0 -222.0 _opencloset)) false false)
              (goto _label :!via `Reset`))))
        (:`B`
          (bind (_direction_2 _opencloset_2) (`Timeline|Timeline_0`)
            (:`Update`
              (`SceneComponent.K2_SetRelativeRotation` (`self.CylinderToRotateLeft`) (`KismetMathLibrary.MakeRotator` 0.0 0.0 (`KismetMathLibrary.Lerp` 130.0 0.0 _opencloset_2)) false false)
              (`SceneComponent.K2_SetRelativeRotation` (`self.CylinderToRotateRight`) (`KismetMathLibrary.MakeRotator` 0.0 0.0 (`KismetMathLibrary.Lerp` -222.0 -92.0 _opencloset_2)) false false)
              (goto _label :!via `Reset`))))))))

(fn `UserConstructionScript`)