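; BP_AlertDownload is an alert beacon that blinks and beeps until the player's download has been initialized.
; A looping timer started on BeginPlay polls the DownloadInitiliazed flag on BP_FirstPersonCharacter.
; While the flag is false, a FlipFlop alternates between dark and a green light with arrow material and beep.
; Once true, each tick of the timer keeps the light off and the mesh on its constant emissive material.
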(event `self.ReceiveBeginPlay`
  (bind _asbp_first_person_character (cast `/Game/Characters/Character/Blueprints/BP_FirstPersonCharacter` (`GameplayStatics.GetPlayerPawn` 0)))
  (set `self.As BP First Person Character` _asbp_first_person_character)
  (`KismetSystemLibrary.K2_SetTimerDelegate` (delegate `DownloadInitialized`) 0.65 true))

(event `DownloadInitialized`
  (bind _pointlight (`self.PointLight`))
  (bind _pointlight_2 (`self.PointLight`))
  (bind _pointlight_3 (`self.PointLight`))
  (if (`/Game/Characters/Character/Blueprints/BP_FirstPersonCharacter.DownloadInitiliazed?` (`self.As BP First Person Character`))
    (`LightComponent.SetLightColor` _pointlight (struct :`R` 1.0 :`G` 1.0 :`B` 1.0 :`A` 1.0) true)
    (`LightComponent.SetIntensity` _pointlight 0.0)
    (`PrimitiveComponent.SetMaterial` (`self.StaticMesh2`) 0 "/Engine/ArtTools/RenderToTexture/Materials/Debug/M_Emissive_Constant.M_Emissive_Constant")
    (else
      (`/Engine/EditorBlueprintResources/StandardMacros.FlipFlop`
        (:`A`
          (`LightComponent.SetLightColor` _pointlight_3 (struct :`R` 1.0 :`G` 1.0 :`B` 1.0 :`A` 1.0) true)
          (`LightComponent.SetIntensity` _pointlight_3 0.0)
          (`PrimitiveComponent.SetMaterial` (`self.StaticMesh2`) 0 "/Engine/ArtTools/RenderToTexture/Materials/Debug/M_Emissive_Constant.M_Emissive_Constant"))
        (:`B`
          (`LightComponent.SetLightColor` _pointlight_2 (struct :`R` 0.065317 :`G` 1.0 :`B` 0.589371 :`A` 1.0) true)
          (`LightComponent.SetIntensity` _pointlight_2 500.0)
          (`PrimitiveComponent.SetMaterial` (`self.StaticMesh2`) 0 "/Engine/VREditor/UI/ArrowMaterial.ArrowMaterial")
          (`GameplayStatics.PlaySoundAtLocation` "/Game/SoundDesign/DecryptionToolSounds/SC_BIP.SC_BIP" (`self.K2_GetActorLocation`) (struct) 1.0 1.0 0.0 null null null null))))))

(fn `UserConstructionScript`)