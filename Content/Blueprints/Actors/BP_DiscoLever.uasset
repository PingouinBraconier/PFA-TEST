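; One-shot disco lever actor that, when interacted with, slides and spawns BP_Light at a fixed world position.
; OnInteract plays a sound and a timeline that lerps Cube11 along local Y, calling SpawnActor on every timeline update rather than once.
; OnLookat applies an overlay highlight and sets the player character's LookAtBool, using a short retriggerable delay to clear both when looking stops.
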(event `self.ReceiveBeginPlay`
  (bind _asbp_first_person_character (cast `/Game/Characters/Character/Blueprints/BP_FirstPersonCharacter` (`GameplayStatics.GetPlayerPawn` 0)))
  (set `self.As BP First Person Character Ref` _asbp_first_person_character))

(event `self.OnInteract`
  (params (InteractingPlayer :type "Character Object Reference"))
  (bind _cube11 (`self.Cube11`))
  (bind (_relativelocation_x _relativelocation_y _relativelocation_z) (`KismetMathLibrary.BreakVector` (`SceneComponent.RelativeLocation` _cube11)))
  (`/Engine/EditorBlueprintResources/StandardMacros.DoOnce` false
    (:`Completed`
      (`GameplayStatics.PlaySound2D` "/Game/SoundDesign/balai_laser/Audio_levier_balai.Audio_levier_balai" 1.0 1.0 0.0 null null)
      (bind (_direction _lever) (`Timeline|Timeline` :!via `PlayFromStart`)
        (:`Update`
          (`SceneComponent.K2_SetRelativeLocation` _cube11 (`KismetMathLibrary.MakeVector` _relativelocation_x (`KismetMathLibrary.Lerp` 20.0 -20.0 _lever) _relativelocation_z) false false)
          (`|SpawnActorFromClass` "/Game/Blueprints/Actors/BP_Light.BP_Light_C" (`KismetMathLibrary.MakeTransform` (-871.0 -3157.0 435.0)) "Undefined" "MultiplyWithRoot" null null))))))

(event `self.OnLookAt`
  (params (Actor :type "Actor Object Reference"))
  (`MeshComponent.SetOverlayMaterial` (`self.Cube11`) "/Game/Materials/M_Overlay.M_Overlay")
  (set `/Game/Characters/Character/Blueprints/BP_FirstPersonCharacter.LookAtBool` true (`self.As BP First Person Character Ref`))
  (`KismetSystemLibrary.RetriggerableDelay` 0.11)
  (`MeshComponent.SetOverlayMaterial` (`self.Cube11`) null)
  (set `/Game/Characters/Character/Blueprints/BP_FirstPersonCharacter.LookAtBool` false (`self.As BP First Person Character Ref`)))

(fn `UserConstructionScript`)