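; Curtain actor that closes on demand and reports its closed state to the first-person player character.
; It caches the player pawn at BeginPlay; the Close! event reveals three curtain components and plays a timeline.
; The timeline lerps only the main Curtain between the Start and End markers, feeding their world locations into a relative-location setter.
; Every update also sets IsClosed and the player's CurtainsClosed flag, so both turn true as movement begins.
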(event `self.ReceiveBeginPlay`
  (bind _asbp_first_person_character (cast `/Game/Characters/Character/Blueprints/BP_FirstPersonCharacter` (`GameplayStatics.GetPlayerPawn` 0)))
  (set `self.As BP First Person Character` _asbp_first_person_character))

(event `Close!`
  (`SceneComponent.SetVisibility` (`self.Curtain`) true false)
  (`SceneComponent.SetVisibility` (`self.Curtain1`) true false)
  (`SceneComponent.SetVisibility` (`self.Curtain2`) true false)
  (set `self.StartLocation` (`SceneComponent.K2_GetComponentLocation` (`self.Start`)))
  (set `self.EndLocation` (`SceneComponent.K2_GetComponentLocation` (`self.End`)))
  (bind (_direction _newtrack_0) (`Timeline|Timeline` :!via `PlayFromStart`)
    (:`Update`
      (`SceneComponent.K2_SetRelativeLocation` (`self.Curtain`) (`KismetMathLibrary.VLerp` (`self.StartLocation`) (`self.EndLocation`) _newtrack_0) false false)
      (set `self.is closed?` true)
      (set `/Game/Characters/Character/Blueprints/BP_FirstPersonCharacter.CurtainsClosed?` true (`self.As BP First Person Character`)))))

(fn `UserConstructionScript`)