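; Robot pod actor that encloses the first-person player to show a menu, then releases them back into gameplay.
; Entering the box closes the front door via timeline, then shows the BP_Menu widget, blends to the widget camera and swaps player input for cursor UI.
; OpenDoor hides the menu, swings the door open with sound and restores player view and input.
; DoorOpened, CanShowWidget and a DoOnce gate re-triggering until the player exits.
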(event `self.ReceiveBeginPlay`
  (bind _returnvalue (`GameplayStatics.GetPlayerController` 0))
  (bind _asbp_first_person_character (cast `/Game/Characters/Character/Blueprints/BP_FirstPersonCharacter` (`GameplayStatics.GetPlayerPawn` 0)))
  (set `self.As BP First Person Character Ref` _asbp_first_person_character)
  (bind _returnvalue_2 (`GameplayStatics.GetActorOfClass` "/Game/Blueprints/Actors/Bp_WidgetCamera.Bp_WidgetCamera_C"))
  (set `self.Camera Ref` _returnvalue_2)
  (set `PlayerController.bShowMouseCursor` true _returnvalue)
  (`WidgetBlueprintLibrary.SetInputMode_GameAndUIEx` _returnvalue (`self.In Widget to Focus`)))

(event `OpenDoor`
  (bind _returnvalue (`GameplayStatics.GetPlayerController` 0))
  (bind _frontdoor (`self.FrontDoor`))
  (bind (_relativerotation_roll _relativerotation_pitch _relativerotation_yaw) (`KismetMathLibrary.BreakRotator` (`SceneComponent.RelativeRotation` _frontdoor)))
  (`/Engine/EditorBlueprintResources/StandardMacros.DoOnce` false :!label _label
    (:`Completed`
      (set `self.DoorOpened` true)
      (set `self.CanShowWidget` false)
      (bind _returnvalue_2 (`GameplayStatics.GetActorOfClass` "/Game/Blueprints/Actors/BP_Menu.BP_Menu_C"))
      (`KismetSystemLibrary.Delay` 0.5)
      (`SceneComponent.SetVisibility` (`/Game/Blueprints/Actors/BP_Menu.Widget` _returnvalue_2) false false)
      (set `PlayerController.bShowMouseCursor` false _returnvalue)
      (`PlayerController.SetViewTargetWithBlend` _returnvalue (`self.As BP First Person Character Ref`) 0.5 "VTBlend_EaseInOut" 2.0 false)
      (`GameplayStatics.PlaySound2D` "/Game/SoundDesign/Ambiant/SW_DoomDoor.SW_DoomDoor" 1.0 1.0 0.0 null null)
      (bind (_direction _newtrack_0) (`Timeline|Timeline` :!via `PlayFromStart`)
        (:`Update`
          (`SceneComponent.K2_SetRelativeRotation` _frontdoor (`KismetMathLibrary.MakeRotator` (`KismetMathLibrary.Lerp` 90.0 -110.0 _newtrack_0) _relativerotation_pitch _relativerotation_yaw) false false)
          (`KismetSystemLibrary.Delay` 1.0)
          (`WidgetBlueprintLibrary.SetInputMode_GameOnly` _returnvalue)
          (`self.EnableInput` (`self.As BP First Person Character Ref`) _returnvalue))))))

(event `self.Box.OnComponentBeginOverlap`
  (params (OverlappedComponent :type "PrimitiveComponent Object Reference") (OtherActor :type "Actor Object Reference") (OtherComp :type "PrimitiveComponent Object Reference") (OtherBodyIndex :type Integer) (bFromSweep :type Boolean) (SweepResult :type "HitResult Structure (by ref)"))
  (bind _returnvalue (`GameplayStatics.GetPlayerController` 0))
  (bind _frontdoor (`self.FrontDoor`))
  (bind (_relativerotation_roll _relativerotation_pitch _relativerotation_yaw) (`KismetMathLibrary.BreakRotator` (`SceneComponent.RelativeRotation` _frontdoor)))
  (if (and (not (`self.DoorOpened`)) (`self.CanShowWidget`))
    (`|ExecutionSequence`
      (:`then_0`
        (set `/Game/Characters/Character/Blueprints/BP_FirstPersonCharacter.IsInThePod` true (`self.As BP First Person Character Ref`))
        (goto _label :!via `Reset`))
      (:`then_1`
        (bind (_direction _newtrack_0) (`Timeline|Timeline_0` :!via `PlayFromStart`)
          (:`Update`
            (`SceneComponent.K2_SetRelativeRotation` _frontdoor (`KismetMathLibrary.MakeRotator` (`KismetMathLibrary.Lerp` -110.0 90.0 _newtrack_0) _relativerotation_pitch _relativerotation_yaw) false false)
            (bind _returnvalue_2 (`GameplayStatics.GetActorOfClass` "/Game/Blueprints/Actors/BP_Menu.BP_Menu_C"))
            (`KismetSystemLibrary.Delay` 1.0)
            (`SceneComponent.SetVisibility` (`/Game/Blueprints/Actors/BP_Menu.Widget` _returnvalue_2) true false)
            (`PlayerController.SetViewTargetWithBlend` _returnvalue (`self.Camera Ref`) 0.5 "VTBlend_EaseInOut" 2.0 false)
            (`WidgetBlueprintLibrary.SetInputMode_GameAndUIEx` _returnvalue (`self.In Widget to Focus`))
            (set `PlayerController.bShowMouseCursor` true _returnvalue)
            (`/Game/Characters/Character/Blueprints/BP_FirstPersonCharacter.Begin` (`self.As BP First Person Character Ref`))
            (`self.DisableInput` (`self.As BP First Person Character Ref`) _returnvalue)))))))

(event `self.Box.OnComponentEndOverlap`
  (params (OverlappedComponent :type "PrimitiveComponent Object Reference") (OtherActor :type "Actor Object Reference") (OtherComp :type "PrimitiveComponent Object Reference") (OtherBodyIndex :type Integer))
  (set `/Game/Characters/Character/Blueprints/BP_FirstPersonCharacter.IsInThePod` false (`self.As BP First Person Character Ref`))
  (set `self.DoorOpened` false)
  (set `self.CanShowWidget` true))

(fn `UserConstructionScript`)