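; BP_Screen is an interactable screen that the player can toggle into and out of with a camera blend.
; OnInteract flip-flops between the BP_CamScreen view and the first-person character, switching input mode, movement, look, mouse and WBP_Cursor visibility.
; It also ducks the BP_RadioButtonPlay audio while the screen is in use.
; OnLookat shows an overlay highlight and ItemRef, which a short retriggerable delay clears once look-at calls stop.
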(event `/Game/Blueprints/Interfaces/BPI_Interaction.OnInteract`
  (params (InteractingPlayer :type "Character Object Reference"))
  (bind _returnvalue (`GameplayStatics.GetPlayerController` 0))
  (`/Engine/EditorBlueprintResources/StandardMacros.FlipFlop`
    (:`A`
      (set `/Game/Characters/Character/Blueprints/BP_FirstPersonCharacter.OnAScreen` true (stale `self.ReceiveBeginPlay` _asbp_first_person_character))
      (`PlayerController.SetViewTargetWithBlend` _returnvalue (stale `self.ReceiveBeginPlay` _returnvalue_2) 0.5 "VTBlend_EaseInOut" 2.0 false)
      (`WidgetBlueprintLibrary.SetInputMode_GameAndUIEx` _returnvalue (`self.In Widget to Focus`))
      (set `CharacterMovementComponent.MaxWalkSpeed` 0.0 (`Character.CharacterMovement` (`self.As BP First Person Character`)))
      (`Controller.SetIgnoreLookInput` _returnvalue true)
      (bind _foundwidgets (`WidgetBlueprintLibrary.GetAllWidgetsOfClass` "/Game/Widgets/HUD/WBP_Cursor.WBP_Cursor_C"))
      (`Widget.SetVisibility` _foundwidgets "Hidden")
      (set `PlayerController.bShowMouseCursor` true _returnvalue)
      (`AudioComponent.SetVolumeMultiplier` (`/Game/Blueprints/InteractiveObjects/Musical/BP_RadioButtonPlay.Audio` (`self.RadioRef`)) 0.05))
    (:`B`
      (set `/Game/Characters/Character/Blueprints/BP_FirstPersonCharacter.OnAScreen` false (stale `self.ReceiveBeginPlay` _asbp_first_person_character))
      (if (not (`/Game/Characters/Character/Blueprints/BP_FirstPersonCharacter.OnAScreen` (stale `self.ReceiveBeginPlay` _asbp_first_person_character)))
        (`PlayerController.SetViewTargetWithBlend` _returnvalue (stale `self.ReceiveBeginPlay` _asbp_first_person_character) 0.5 "VTBlend_EaseInOut" 2.0 false)
        (`KismetSystemLibrary.Delay` 0.5)
        (bind _foundwidgets_2 (`WidgetBlueprintLibrary.GetAllWidgetsOfClass` "/Game/Widgets/HUD/WBP_Cursor.WBP_Cursor_C"))
        (`Widget.SetVisibility` _foundwidgets_2 "Visible")
        (`WidgetBlueprintLibrary.SetInputMode_GameOnly` _returnvalue)
        (`Controller.SetIgnoreLookInput` _returnvalue false)
        (set `CharacterMovementComponent.MaxWalkSpeed` 500.0 (`Character.CharacterMovement` (`self.As BP First Person Character`)))
        (set `PlayerController.bShowMouseCursor` false _returnvalue)
        (`AudioComponent.SetVolumeMultiplier` (`/Game/Blueprints/InteractiveObjects/Musical/BP_RadioButtonPlay.Audio` (`self.RadioRef`)) 1.0)))))

(event `self.ReceiveBeginPlay`
  (bind _asbp_first_person_character (cast `/Game/Characters/Character/Blueprints/BP_FirstPersonCharacter` (`GameplayStatics.GetPlayerPawn` 0)))
  (bind _returnvalue (`GameplayStatics.GetActorOfClass` "/Game/Blueprints/InteractiveObjects/Musical/BP_RadioButtonPlay.BP_RadioButtonPlay_C"))
  (set `self.RadioRef` _returnvalue)
  (set `self.As BP First Person Character` _asbp_first_person_character)
  (bind _returnvalue_2 (`GameplayStatics.GetActorOfClass` "/Game/Blueprints/Actors/BP_CamScreen.BP_CamScreen_C")))

(event `/Game/Blueprints/Interfaces/BPI_Interaction.OnLookAt`
  (params (Actor :type "Actor Object Reference"))
  (`MeshComponent.SetOverlayMaterial` (`self.Cube`) "/Game/Materials/M_Overlay.M_Overlay")
  (`MeshComponent.SetOverlayMaterial` (`self.Cube1`) "/Game/Materials/M_Overlay.M_Overlay")
  (`SceneComponent.SetVisibility` (`self.ItemRef`) true false)
  (`KismetSystemLibrary.RetriggerableDelay` 0.11)
  (`MeshComponent.SetOverlayMaterial` (`self.Cube1`) null)
  (`MeshComponent.SetOverlayMaterial` (`self.Cube`) null)
  (`SceneComponent.SetVisibility` (`self.ItemRef`) false false))

(fn `UserConstructionScript`)