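; BP_Book is an actor representing a book, with cover, spine, back cover, a picture plane and a title text.
; On BeginPlay it applies one material to the cover, spine and back cover, and a separate picture material to the plane.
; It sets the text render to its Title variable, so these visuals appear only at runtime, as the construction script is empty.
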(event `self.ReceiveBeginPlay`
  (`PrimitiveComponent.SetMaterial` (`self.Couverture`) 0 (`self.Material`))
  (`PrimitiveComponent.SetMaterial` (`self.Tranche`) 0 (`self.Material`))
  (`PrimitiveComponent.SetMaterial` (`self.4eDeCouverture`) 0 (`self.Material`))
  (`PrimitiveComponent.SetMaterial` (`self.Plane`) 0 (`self.Material_Picture`))
  (`TextRenderComponent.K2_SetText` (`self.TextRender`) (`self.Title`)))

(fn `UserConstructionScript`)