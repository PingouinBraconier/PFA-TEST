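; Robot bed actor that sets up the main menu and has a hinged cylinder that opens like a door.
; BeginPlay creates and stores the main menu widget, shows the cursor and switches input to game and UI.
; OpenDoor runs once, playing a timeline that pitches the cylinder open.
; Each timeline update also sets game-only input while keeping the cursor flag on.
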(event `self.ReceiveBeginPlay`
  (bind _returnvalue (`GameplayStatics.GetPlayerController` 0))
  (bind _returnvalue_2 (`|CreateWidget` "/Game/Widgets/Menu/WBP_MainMenu.WBP_MainMenu_C"))
  (set `self.MainMenu` _returnvalue_2)
  (set `PlayerController.bShowMouseCursor` true _returnvalue)
  (`WidgetBlueprintLibrary.SetInputMode_GameAndUIEx` _returnvalue (`self.In Widget to Focus`)))

(event `OpenDoor`
  (bind _returnvalue (`GameplayStatics.GetPlayerController` 0))
  (`/Engine/EditorBlueprintResources/StandardMacros.DoOnce` false
    (:`Completed`
      (bind (_direction _newtrack_0) (`Timeline|Timeline`)
        (:`Update`
          (`SceneComponent.K2_SetRelativeRotation` (`self.CylinderOpen`) (`KismetMathLibrary.MakeRotator` 0.0 (`KismetMathLibrary.Lerp` 0.0 -110.0 _newtrack_0)) false false)
          (`WidgetBlueprintLibrary.SetInputMode_GameOnly` _returnvalue)
          (set `PlayerController.bShowMouseCursor` true _returnvalue))))))

(fn `UserConstructionScript`)