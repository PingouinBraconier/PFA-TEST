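; BP_Lever is an interactable lever that closes the curtain in the level, usable once.
; OnInteract finds the Bp_Curtain actor, then plays a DoOnce-gated timeline that slides a lever piece along Y and calls the curtain's Close on every update.
; OnLookat applies an overlay material, shows a widget and sets the first-person character's look-at flag.
; A short retriggerable delay clears these once the look-at calls stop.
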(event `self.ReceiveBeginPlay`
  (bind _asbp_first_person_character (cast `/Game/Characters/Character/Blueprints/BP_FirstPersonCharacter` (`GameplayStatics.GetPlayerPawn` 0)))
  (set `self.As BP First Person Character Ref` _asbp_first_person_character))

(event `/Game/Blueprints/Interfaces/BPI_Interaction.OnInteract`
  (params (InteractingPlayer :type "Character Object Reference"))
  (bind _cube11 (`self.Cube11`))
  (bind (_relativelocation_x _relativelocation_y _relativelocation_z) (`KismetMathLibrary.BreakVector` (`SceneComponent.RelativeLocation` _cube11)))
  (bind _returnvalue (`GameplayStatics.GetActorOfClass` "/Game/Blueprints/Actors/Bp_Curtain.Bp_Curtain_C"))
  (bind _output_get (set `self.Curtain Ref` _returnvalue))
  (`/Engine/EditorBlueprintResources/StandardMacros.DoOnce` false
    (:`Completed`
      (bind (_direction _lever) (`Timeline|Timeline` :!via `PlayFromStart`)
        (:`Update`
          (`SceneComponent.K2_SetRelativeLocation` _cube11 (`KismetMathLibrary.MakeVector` _relativelocation_x (`KismetMathLibrary.Lerp` 20.0 -20.0 _lever) _relativelocation_z) false false)
          (`/Game/Blueprints/Actors/Bp_Curtain.Close!` _output_get))))))

(event `/Game/Blueprints/Interfaces/BPI_Interaction.OnLookAt`
  (params (Actor :type "Actor Object Reference"))
  (`MeshComponent.SetOverlayMaterial` (`self.Cube6`) "/Game/Materials/M_Overlay.M_Overlay")
  (`MeshComponent.SetOverlayMaterial` (`self.Cube7`) "/Game/Materials/M_Overlay.M_Overlay")
  (`MeshComponent.SetOverlayMaterial` (`self.Cube8`) "/Game/Materials/M_Overlay.M_Overlay")
  (`MeshComponent.SetOverlayMaterial` (`self.Cube5`) "/Game/Materials/M_Overlay.M_Overlay")
  (`MeshComponent.SetOverlayMaterial` (`self.Cube1`) "/Game/Materials/M_Overlay.M_Overlay")
  (`MeshComponent.SetOverlayMaterial` (`self.Cube2`) "/Game/Materials/M_Overlay.M_Overlay")
  (`MeshComponent.SetOverlayMaterial` (`self.Cube3`) "/Game/Materials/M_Overlay.M_Overlay")
  (`MeshComponent.SetOverlayMaterial` (`self.Cube4`) "/Game/Materials/M_Overlay.M_Overlay")
  (`MeshComponent.SetOverlayMaterial` (`self.Cube10`) "/Game/Materials/M_Overlay.M_Overlay")
  (`SceneComponent.SetVisibility` (`self.Widget`) true false)
  (set `/Game/Characters/Character/Blueprints/BP_FirstPersonCharacter.LookAtBool` true (`self.As BP First Person Character Ref`))
  (`KismetSystemLibrary.RetriggerableDelay` 0.11)
  (`MeshComponent.SetOverlayMaterial` (`self.Cube6`) null)
  (`MeshComponent.SetOverlayMaterial` (`self.Cube7`) null)
  (`MeshComponent.SetOverlayMaterial` (`self.Cube8`) null)
  (`MeshComponent.SetOverlayMaterial` (`self.Cube5`) null)
  (`MeshComponent.SetOverlayMaterial` (`self.Cube1`) null)
  (`MeshComponent.SetOverlayMaterial` (`self.Cube2`) null)
  (`MeshComponent.SetOverlayMaterial` (`self.Cube3`) null)
  (`MeshComponent.SetOverlayMaterial` (`self.Cube4`) null)
  (`MeshComponent.SetOverlayMaterial` (`self.Cube10`) null)
  (`SceneComponent.SetVisibility` (`self.Widget`) false false)
  (set `/Game/Characters/Character/Blueprints/BP_FirstPersonCharacter.LookAtBool` false (`self.As BP First Person Character Ref`)))

(fn `UserConstructionScript`)