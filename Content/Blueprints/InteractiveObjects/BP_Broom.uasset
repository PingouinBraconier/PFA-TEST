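; BP_Broom is an interactable broom that the player picks up and puts back, blocked while the player holds TapeObtained.
; Interacting toggles the character's broom state and plays timelines that lerp the mesh between its starting transform and the player's PlayerBroom.
; Delays handle visibility, collision and a brief re-interaction lockout.
; Looking at it applies an overlay material, cleared by a retriggerable delay once the look events stop.
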(event `self.ReceiveBeginPlay`
  (bind _asbp_first_person_character (cast `/Game/Characters/Character/Blueprints/BP_FirstPersonCharacter` (`GameplayStatics.GetPlayerPawn` 0)))
  (set `self.As BP First Person Character Ref` _asbp_first_person_character)
  (set `self.StartBroomTransform` (`SceneComponent.K2_GetComponentToWorld` (`self.Broom`))))

(event `/Game/Blueprints/Interfaces/BPI_Interaction.OnInteract`
  (params (InteractingPlayer :type "Character Object Reference"))
  (bind _as_bp_first_person_character_ref (`self.As BP First Person Character Ref`))
  (if (`/Game/Characters/Character/Blueprints/BP_FirstPersonCharacter.TapeObtained` (`self.As BP First Person Character Ref`))
    _
    (elif (`self.IsAnimatingBroom`)
      _
      (elif (`/Game/Characters/Character/Blueprints/BP_FirstPersonCharacter.BroomObtained` (`self.As BP First Person Character Ref`))
        (`GameplayStatics.PlaySound2D` "/Engine/VREditor/Sounds/UI/Object_PickUp.Object_PickUp" 1.0 1.0 0.0 null null)
        (`/Game/Characters/Character/Blueprints/BP_FirstPersonCharacter.NoBroom!` _as_bp_first_person_character_ref)
        (`KismetSystemLibrary.Delay` 0.5)
        (`SceneComponent.SetVisibility` (`self.Broom`) true false)
        (set `self.IsAnimatingBroom` true)
        (`self.BroomCooldown`)
        (bind (_direction _alpha) (`Timeline|Timeline` :!via `ReverseFromEnd`)
          (:`Update`
            (bind _returnvalue (`KismetMathLibrary.TLerp` (`self.StartBroomTransform`) (`SceneComponent.K2_GetComponentToWorld` (`/Game/Characters/Character/Blueprints/BP_FirstPersonCharacter.PlayerBroom` _as_bp_first_person_character_ref)) _alpha))
            (`SceneComponent.K2_SetWorldLocation` (`self.Broom`) (.location _returnvalue) false false)
            (`SceneComponent.K2_SetWorldRotation` (`self.Broom`) (`KismetMathLibrary.MakeRotator` (.roll (.rotation _returnvalue)) (.pitch (.rotation _returnvalue)) (.yaw (.rotation _returnvalue))) false false)
            (`KismetSystemLibrary.Delay` 0.25)
            (`PrimitiveComponent.SetCollisionEnabled` (`self.Broom`) "QueryAndPhysics")))
        (else
          (`GameplayStatics.PlaySound2D` "/Engine/VREditor/Sounds/UI/Object_PickUp.Object_PickUp" 1.0 1.0 0.0 null null)
          (`/Game/Characters/Character/Blueprints/BP_FirstPersonCharacter.Broom!` (`self.As BP First Person Character Ref`))
          (set `self.IsAnimatingBroom` true)
          (`self.BroomCooldown`)
          (`PrimitiveComponent.SetCollisionEnabled` (`self.Broom`) "NoCollision")
          (bind (_direction_2 _alpha_2) (`Timeline|Tl_Broom` :!via `PlayFromStart`)
            (:`Update`
              (bind _returnvalue_2 (`KismetMathLibrary.TLerp` (`self.StartBroomTransform`) (`SceneComponent.K2_GetComponentToWorld` (`/Game/Characters/Character/Blueprints/BP_FirstPersonCharacter.PlayerBroom` (`self.As BP First Person Character Ref`))) _alpha_2))
              (`SceneComponent.K2_SetWorldLocation` (`self.Broom`) (.location _returnvalue_2) false false)
              (`SceneComponent.K2_SetWorldRotation` (`self.Broom`) (`KismetMathLibrary.MakeRotator` (.roll (.rotation _returnvalue_2)) (.pitch (.rotation _returnvalue_2)) (.yaw (.rotation _returnvalue_2))) false false)
              (`PrimitiveComponent.SetCollisionEnabled` (`self.Broom`) "NoCollision")
              (`self.Visible`))))))))

(event `BroomCooldown`
  (`KismetSystemLibrary.Delay` 0.25)
  (set `self.IsAnimatingBroom` false))

(event `Visible`
  (`KismetSystemLibrary.Delay` 0.25)
  (`SceneComponent.SetVisibility` (`self.Broom`) false false))

(event `/Game/Blueprints/Interfaces/BPI_Interaction.OnLookAt`
  (params (Actor :type "Actor Object Reference"))
  (`MeshComponent.SetOverlayMaterial` (`self.Broom`) "/Game/Materials/M_Overlay.M_Overlay")
  (`KismetSystemLibrary.RetriggerableDelay` 0.11)
  (`MeshComponent.SetOverlayMaterial` (`self.Broom`) null))

(fn `UserConstructionScript`)