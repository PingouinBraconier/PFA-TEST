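; Interactive lever that opens and closes the broom closet found in the level at BeginPlay.
; OnInteract toggles IsOpen, plays a sound and runs the Open timeline forward or backward to rotate the lever parts.
; The timeline update passes through a 1.5-second Delay, then calls Open or Close on the closet; CloseWindow forces the closing path.
; OnLookat applies a highlight overlay that a short RetriggerableDelay clears once calls stop.
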(event `self.ReceiveBeginPlay`
  (bind _returnvalue (`GameplayStatics.GetActorOfClass` "/Game/Blueprints/InteractiveObjects/BP_BroomCloset.BP_BroomCloset_C"))
  (set `self.BroomCloset Ref` _returnvalue)
  (set `self.EndRotation` (`KismetMathLibrary.MakeRotator` 0.0 (- 0.0 70.0))))

(event `/Game/Blueprints/Interfaces/BPI_Interaction.OnLookAt`
  (params (Actor :type "Actor Object Reference"))
  (`MeshComponent.SetOverlayMaterial` (`self.Cylinder`) "/Game/Materials/M_Overlay.M_Overlay")
  (`MeshComponent.SetOverlayMaterial` (`self.Cylinder1`) "/Game/Materials/M_Overlay.M_Overlay")
  (`MeshComponent.SetOverlayMaterial` (`self.Cylinder2`) "/Game/Materials/M_Overlay.M_Overlay")
  (`MeshComponent.SetOverlayMaterial` (`self.Cube`) "/Game/Materials/M_Overlay.M_Overlay")
  (`MeshComponent.SetOverlayMaterial` (`self.Cube1`) "/Game/Materials/M_Overlay.M_Overlay")
  (`KismetSystemLibrary.RetriggerableDelay` 0.11)
  (`MeshComponent.SetOverlayMaterial` (`self.Cylinder`) null)
  (`MeshComponent.SetOverlayMaterial` (`self.Cylinder1`) null)
  (`MeshComponent.SetOverlayMaterial` (`self.Cylinder2`) null)
  (`MeshComponent.SetOverlayMaterial` (`self.Cube`) null)
  (`MeshComponent.SetOverlayMaterial` (`self.Cube1`) null))

(event `/Game/Blueprints/Interfaces/BPI_Interaction.OnInteract`
  (params (InteractingPlayer :type "Character Object Reference"))
  (bind _broomcloset_ref (`self.BroomCloset Ref`))
  (if (`self.IsOpen`)
    (set `self.IsOpen` false :!label _label)
    (`GameplayStatics.PlaySound2D` "/Game/SoundDesign/balai_laser/Audio_levier_balai.Audio_levier_balai" 1.0 1.0 0.0 null null)
    (bind (_direction _switch) (`Timeline|Open` :!via `ReverseFromEnd` :!label _label_2)
      (:`Update`
        (`SceneComponent.K2_SetRelativeRotation` (`self.Cylinder`) (`KismetMathLibrary.RLerp` (`self.StartRotation`) (`self.EndRotation`) _switch) false false)
        (`SceneComponent.K2_SetRelativeRotation` (`self.Cylinder1`) (`KismetMathLibrary.RLerp` (`self.StartRotation`) (`self.EndRotation`) _switch) false false)
        (`SceneComponent.K2_SetRelativeRotation` (`self.GhostSupport`) (`KismetMathLibrary.RLerp` (`self.StartRotation`) (`self.EndRotation`) _switch) false false)
        (`KismetSystemLibrary.Delay` 1.5)
        (if (`self.IsOpen`)
          (`/Game/Blueprints/InteractiveObjects/BP_BroomCloset.Open` _broomcloset_ref)
          (else
            (`/Game/Blueprints/InteractiveObjects/BP_BroomCloset.Close` _broomcloset_ref)))))
    (else
      (set `self.IsOpen` true)
      (`GameplayStatics.PlaySound2D` "/Game/SoundDesign/balai_laser/Audio_levier_balai.Audio_levier_balai" 1.0 1.0 0.0 null null)
      (goto _label_2 :!via `PlayFromStart`))))

(event `CloseWindow`
  (goto _label))

(fn `UserConstructionScript`)