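; BP_RadioButtonNext is an interactable radio button that starts and stops music.
; OnInteract plays the Press timeline, which lowers the Cylinder mesh along Z.
; The TurnOnOff toggle runs on every timeline update, alternately spawning a 2D sound from MusicList at MusicNumber and stopping it through MusicRef.
; Despite the name, MusicNumber never changes here, and the player character reference cached on BeginPlay is unused.
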(event `self.ReceiveBeginPlay`
  (bind _asbp_first_person_character (cast `/Game/Characters/Character/Blueprints/BP_FirstPersonCharacter` (`GameplayStatics.GetPlayerPawn` 0)))
  (set `self.As BP First Person Character Ref` _asbp_first_person_character))

(event `self.OnInteract`
  (params (InteractingPlayer :type "Character Object Reference"))
  (bind _music_ref (`self.Music Ref`))
  (bind (_relativelocation_x _relativelocation_y) (`KismetMathLibrary.BreakVector` (`SceneComponent.RelativeLocation` (`self.Cylinder`))))
  (bind (_direction _press) (`Timeline|Press` :!via `PlayFromStart`)
    (:`Update`
      (`SceneComponent.K2_SetRelativeLocation` (`self.Cylinder`) (`KismetMathLibrary.MakeVector` _relativelocation_x _relativelocation_y (`KismetMathLibrary.Lerp` 100.0 80.0 _press)) false false)
      (if (`self.Turn On/Off`)
        (set `self.Turn On/Off` false)
        (`/Engine/EditorBlueprintResources/StandardMacros.IsValid` _music_ref
          (:`Is Valid`
            (`AudioComponent.Stop` _music_ref)))
        (else
          (set `self.Turn On/Off` true)
          (`self.Play`))))))

(event `Play`
  (bind _returnvalue (`GameplayStatics.SpawnSound2D` (`|GetArrayItem` (`self.MusicList`) (`self.MusicNumber`)) 0.5 1.0 0.0 null))
  (set `self.Music Ref` _returnvalue))

(fn `UserConstructionScript`)