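; BP_Decryption is an interactive decryption object that triggers the Enter function on the first-person player character when interacted with.
; It caches the player character reference on BeginPlay.
; OnInteract is gated by a cooldown flag and a DoOnce, which a short delayed cooldown event clears and resets so the object can be used again without rapid repeat triggers.
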(event `self.ReceiveBeginPlay`
  (bind _asbp_first_person_character (cast `/Game/Characters/Character/Blueprints/BP_FirstPersonCharacter` (`GameplayStatics.GetPlayerPawn` 0)))
  (set `self.As BP First Person Character Ref` _asbp_first_person_character))

(event `/Game/Blueprints/InteractiveObjects/BPI_Interaction.OnInteract`
  (params (InteractingPlayer :type "Character Object Reference"))
  (if (not (`self.OnCooldown`))
    (`/Engine/EditorBlueprintResources/StandardMacros.DoOnce` false :!label _label
      (:`Completed`
        (`/Game/Characters/Character/Blueprints/BP_FirstPersonCharacter.Enter` (`self.As BP First Person Character Ref`))
        (set `self.OnCooldown` true)
        (`self.Cooldownm`)))))

(event `Cooldownm`
  (`KismetSystemLibrary.Delay` 1.0)
  (set `self.OnCooldown` false)
  (goto _label :!via `Reset`))

(fn `UserConstructionScript`)