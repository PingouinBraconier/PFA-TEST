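; Interactable radio play button that starts music at BeginPlay and toggles it on interaction.
; OnInteract animates the cylinder press through a timeline whose update also flips the on/off state and starts a short cooldown.
; Play spawns the 2D track selected by the first-person character's MusicList and MusicNumber.
; A looping timer stops music while the player is decrypting, otherwise respawns it whenever the audio reference is invalid, without checking the toggle.
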(event `self.ReceiveBeginPlay`
  (bind _asbp_first_person_character (cast `/Game/Characters/Character/Blueprints/BP_FirstPersonCharacter` (`GameplayStatics.GetPlayerPawn` 0)))
  (set `self.As BP First Person Character Ref` _asbp_first_person_character)
  (`self.Play`))

(event `/Game/Blueprints/Interfaces/BPI_Interaction.OnInteract`
  (params (InteractingPlayer :type "Character Object Reference"))
  (bind _music_ref (`self.Music Ref`))
  (bind (_relativelocation_x _relativelocation_y) (`KismetMathLibrary.BreakVector` (`SceneComponent.RelativeLocation` (`self.Cylinder`))))
  (if (not (`self.OnCooldown`))
    (bind (_direction _press) (`Timeline|Press` :!via `PlayFromStart`)
      (:`Update`
        (`SceneComponent.K2_SetRelativeLocation` (`self.Cylinder`) (`KismetMathLibrary.MakeVector` _relativelocation_x _relativelocation_y (`KismetMathLibrary.Lerp` 100.0 80.0 _press)) false false)
        (set `self.OnCooldown` true)
        (`self.Cooldown`)
        (if (`self.Turn On/Off`)
          (set `self.Turn On/Off` false)
          (`/Engine/EditorBlueprintResources/StandardMacros.IsValid` _music_ref
            (:`Is Valid`
              (`AudioComponent.Stop` _music_ref)))
          (else
            (set `self.Turn On/Off` true)
            (`self.Play`)))))))

(event `Cooldown`
  (`KismetSystemLibrary.Delay` 1.5)
  (set `self.OnCooldown` false))

(event `Play`
  (bind _as_bp_first_person_character_ref (`self.As BP First Person Character Ref`))
  (bind _returnvalue (`GameplayStatics.SpawnSound2D` (`|GetArrayItem` (`/Game/Characters/Character/Blueprints/BP_FirstPersonCharacter.MusicList` _as_bp_first_person_character_ref) (`/Game/Characters/Character/Blueprints/BP_FirstPersonCharacter.MusicNumber` _as_bp_first_person_character_ref)) 0.5 1.0 0.0 null :!label _label))
  (set `self.Music Ref` _returnvalue)
  (`KismetSystemLibrary.K2_SetTimerDelegate` (delegate `Stop`) 0.5 true))

(event `Stop`
  (bind _music_ref (`self.Music Ref`))
  (if (`/Game/Characters/Character/Blueprints/BP_FirstPersonCharacter.IsDecrypting` (`self.As BP First Person Character Ref`))
    (`/Engine/EditorBlueprintResources/StandardMacros.IsValid` _music_ref
      (:`Is Valid`
        (`AudioComponent.Stop` _music_ref)))
    (else
      (`/Engine/EditorBlueprintResources/StandardMacros.IsValid` _music_ref
        (:`Is Not Valid`
          (goto _label))))))

(fn `UserConstructionScript`)