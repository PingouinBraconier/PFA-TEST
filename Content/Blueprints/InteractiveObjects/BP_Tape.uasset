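; Interactable tape that the player picks up or puts back, unless they hold the broom.
; OnInteract checks the first-person character's TapeObtained flag, then timelines lerp the mesh between its start transform and the player's PlayerTape component.
; Visibility and collision switch off on pickup and return on put-back, with a short cooldown flag between interactions.
; OnLookat shows ItemRef and an overlay highlight, cleared by a retriggerable delay.
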(event `self.ReceiveBeginPlay`
  (bind _asbp_first_person_character (cast `/Game/Characters/Character/Blueprints/BP_FirstPersonCharacter` (`GameplayStatics.GetPlayerPawn` 0)))
  (set `self.As BP First Person Character Ref` _asbp_first_person_character)
  (set `self.StartTapeTransform` (`SceneComponent.K2_GetComponentToWorld` (`self.Tape`))))

(event `/Game/Blueprints/Interfaces/BPI_Interaction.OnInteract`
  (params (InteractingPlayer :type "Character Object Reference"))
  (bind _tape (`self.Tape`))
  (bind _as_bp_first_person_character_ref (`self.As BP First Person Character Ref`))
  (if (`/Game/Characters/Character/Blueprints/BP_FirstPersonCharacter.BroomObtained` (`self.As BP First Person Character Ref`))
    _
    (elif (`self.IsAnimatingTape`)
      _
      (elif (`/Game/Characters/Character/Blueprints/BP_FirstPersonCharacter.TapeObtained` (`self.As BP First Person Character Ref`))
        (`GameplayStatics.PlaySound2D` "/Engine/VREditor/Sounds/UI/Object_PickUp.Object_PickUp" 1.0 1.0 0.0 null null)
        (`SceneComponent.SetVisibility` (`self.Tape`) true false)
        (`SceneComponent.SetVisibility` (`self.Sphere1`) true false)
        (set `self.IsAnimatingTape` true)
        (`self.TapeCooldown`)
        (`/Game/Characters/Character/Blueprints/BP_FirstPersonCharacter.NoTape!` _as_bp_first_person_character_ref)
        (bind (_direction _alpha) (`Timeline|Timeline` :!via `ReverseFromEnd`)
          (:`Update`
            (bind _returnvalue (`KismetMathLibrary.TLerp` (`self.StartTapeTransform`) (`SceneComponent.K2_GetComponentToWorld` (`/Game/Characters/Character/Blueprints/BP_FirstPersonCharacter.PlayerTape` _as_bp_first_person_character_ref)) _alpha))
            (`SceneComponent.K2_SetWorldTransform` _tape (`KismetMathLibrary.MakeTransform` (.location _returnvalue) (`KismetMathLibrary.MakeRotator` (.roll (.rotation _returnvalue)) 0.0 (.yaw (.rotation _returnvalue))) (.scale _returnvalue)) false false)
            (`KismetSystemLibrary.Delay` 0.1)
            (`PrimitiveComponent.SetCollisionEnabled` (`self.Tape`) "QueryAndPhysics")
            (`PrimitiveComponent.SetCollisionEnabled` (`self.Sphere1`) "QueryAndPhysics")))
        (else
          (`GameplayStatics.PlaySound2D` "/Engine/VREditor/Sounds/UI/Object_PickUp.Object_PickUp" 1.0 1.0 0.0 null null)
          (`/Game/Characters/Character/Blueprints/BP_FirstPersonCharacter.Tape!` (`self.As BP First Person Character Ref`))
          (`PrimitiveComponent.SetCollisionEnabled` (`self.Tape`) "NoCollision")
          (`PrimitiveComponent.SetCollisionEnabled` (`self.Sphere1`) "NoCollision")
          (set `self.IsAnimatingTape` true)
          (`self.TapeCooldown`)
          (bind (_direction_2 _alpha_2) (`Timeline|Timeline_0` :!via `PlayFromStart`)
            (:`Update`
              (bind _returnvalue_2 (`KismetMathLibrary.TLerp` (`self.StartTapeTransform`) (`SceneComponent.K2_GetComponentToWorld` (`/Game/Characters/Character/Blueprints/BP_FirstPersonCharacter.PlayerTape` (`self.As BP First Person Character Ref`))) _alpha_2))
              (`SceneComponent.K2_SetWorldTransform` _tape (`KismetMathLibrary.MakeTransform` (.location _returnvalue_2) (`KismetMathLibrary.MakeRotator` (.roll (.rotation _returnvalue_2)) 0.0 (.yaw (.rotation _returnvalue_2))) (.scale _returnvalue_2)) false false)
              (`PrimitiveComponent.SetCollisionEnabled` (`self.Tape`) "NoCollision")
              (`PrimitiveComponent.SetCollisionEnabled` (`self.Sphere1`) "NoCollision")
              (`self.Visible`))))))))

(event `TapeCooldown`
  (`KismetSystemLibrary.Delay` 0.1)
  (set `self.IsAnimatingTape` false))

(event `Visible`
  (`KismetSystemLibrary.Delay` 0.1)
  (`SceneComponent.SetVisibility` (`self.Tape`) false false)
  (`SceneComponent.SetVisibility` (`self.Sphere1`) false false))

(event `/Game/Blueprints/Interfaces/BPI_Interaction.OnLookAt`
  (params (Actor :type "Actor Object Reference"))
  (`SceneComponent.SetVisibility` (`self.ItemRef`) true false)
  (`MeshComponent.SetOverlayMaterial` (`self.Tape`) "/Game/Materials/M_Overlay.M_Overlay")
  (`KismetSystemLibrary.RetriggerableDelay` 0.11)
  (`SceneComponent.SetVisibility` (`self.ItemRef`) false false)
  (`MeshComponent.SetOverlayMaterial` (`self.Tape`) null))

(fn `UserConstructionScript`)