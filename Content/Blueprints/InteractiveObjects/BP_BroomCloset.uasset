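; Broom closet interactive object that opens and closes behind a laser barrier, with sound cues.
; Open animates the window material's opacity and disables its collision, then retracts the sheathes and laser pivots by scale lerps.
; Close reverses that order and restores collision, with both sequences chaining timelines through Delays on Update pins and guarded by IsOpen.
; OnInteract is empty, while BroomCooldown and Visible only delay.
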(event `self.ReceiveBeginPlay`
  (`GameplayStatics.PlaySound2D` "/Game/SoundDesign/Ambiant/SC_AmbiantNoise.SC_AmbiantNoise" 1.5 1.0 0.0 null null)
  (bind _asbp_first_person_character (cast `/Game/Characters/Character/Blueprints/BP_FirstPersonCharacter` (`GameplayStatics.GetPlayerPawn` 0)))
  (set `self.As BP First Person Character Ref` _asbp_first_person_character)
  (bind _returnvalue (`PrimitiveComponent.CreateDynamicMaterialInstance` (`self.Window`) 0 "/Game/Blueprints/InteractiveObjects/M_LaserCloset.M_LaserCloset" "None"))
  (set `self.LaserMat` _returnvalue))

(event `Close`
  (if (`self.IsOpen`)
    (set `self.IsOpen` false)
    (`GameplayStatics.PlaySound2D` "/Game/SoundDesign/balai_laser/Audio_balai_release_Cue.Audio_balai_release_Cue" 1.0 1.0 0.0 null null)
    (bind (_direction _out) (`Timeline|RetractReverse`)
      (:`Update`
        (`SceneComponent.SetRelativeScale3D` (`self.LaserPivot1`) (`KismetMathLibrary.VLerp` (0.0 0.0 0.0) (`self.StartScale`) _out))
        (`SceneComponent.SetRelativeScale3D` (`self.LaserPivot2`) (`KismetMathLibrary.VLerp` (0.0 0.0 0.0) (`self.StartScale`) _out))
        (`KismetSystemLibrary.Delay` 1.0)
        (bind (_direction_2 _retract) (`Timeline|Timeline` :!via `PlayFromStart`)
          (:`Update`
            (`SceneComponent.SetRelativeScale3D` (`self.Sheathe`) (`KismetMathLibrary.VLerp` (1.0 1.0 0.0) (`self.SheatheScale`) _retract))
            (`SceneComponent.SetRelativeScale3D` (`self.Sheathe1`) (`KismetMathLibrary.VLerp` (1.0 1.0 0.0) (`self.SheatheScale`) _retract))
            (`KismetSystemLibrary.Delay` 1.0)
            (bind (_direction_3 _closing) (`Timeline|Closing` :!via `PlayFromStart`)
              (:`Update`
                (`MaterialInstanceDynamic.SetScalarParameterValue` (`self.LaserMat`) "Opacity" _closing)
                (`PrimitiveComponent.SetCollisionEnabled` (`self.Window`) "QueryAndPhysics"))))
          (:`Finished`
            (`GameplayStatics.SpawnSound2D` "/Game/SoundDesign/balai_laser/Audio_ouverture_balai_Cue.Audio_ouverture_balai_Cue" 2.0 1.0 0.0 null)))))))

(event `Open`
  (if (not (`self.IsOpen`))
    (set `self.IsOpen` true)
    (`GameplayStatics.PlaySound2D` "/Game/SoundDesign/balai_laser/Audio_ouverture_balai_Cue.Audio_ouverture_balai_Cue" 2.0 1.0 0.0 null null)
    (bind (_direction _opening) (`Timeline|Opening`)
      (:`Update`
        (`MaterialInstanceDynamic.SetScalarParameterValue` (`self.LaserMat`) "Opacity" _opening)
        (`PrimitiveComponent.SetCollisionEnabled` (`self.Window`) "NoCollision")
        (`KismetSystemLibrary.Delay` 1.5)
        (bind (_direction_2 _retract) (`Timeline|Retract` :!via `PlayFromStart`)
          (:`Update`
            (`SceneComponent.SetRelativeScale3D` (`self.Sheathe`) (`KismetMathLibrary.VLerp` (`self.SheatheScale`) (1.0 1.0 0.0) _retract))
            (`SceneComponent.SetRelativeScale3D` (`self.Sheathe1`) (`KismetMathLibrary.VLerp` (`self.SheatheScale`) (1.0 1.0 0.0) _retract))
            (`KismetSystemLibrary.Delay` 1.0)
            (bind (_direction_3 _out) (`Timeline|LaserOn/Out` :!via `PlayFromStart`)
              (:`Update`
                (`SceneComponent.SetRelativeScale3D` (`self.LaserPivot1`) (`KismetMathLibrary.VLerp` (`self.StartScale`) (0.0 0.0 0.0) _out))
                (`SceneComponent.SetRelativeScale3D` (`self.LaserPivot2`) (`KismetMathLibrary.VLerp` (`self.StartScale`) (0.0 0.0 0.0) _out)))))))
      (:`Finished`
        (`GameplayStatics.PlaySound2D` "/Game/SoundDesign/balai_laser/Audio_balai_release_Cue.Audio_balai_release_Cue" 1.0 1.0 0.0 null null)))))

(event `self.OnInteract`
  (params (InteractingPlayer :type "Character Object Reference")))

(event `BroomCooldown`
  (`KismetSystemLibrary.Delay` 0.25))

(event `Visible`
  (`KismetSystemLibrary.Delay` 0.25))

(fn `UserConstructionScript`)